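; Player ship Blueprint for a Space Invaders game, handling shooting and death.
; Tick caches the game mode and, while Fire is set, spawns a player projectile, using a DoOnce reset by a Delay as the cooldown.
; Trigger overlap with an alien projectile spawns an explosion, then destroys both the player and that projectile.
; BeginPlay initializes Speed, but no movement logic appears in these graphs.
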(event `self.ReceiveTick`
  (params (DeltaSeconds :type "Float (single-precision)"))
  (bind _asspace_invaders_game_mode (cast `/Game/Blueprints/SpaceInvaders_GameMode` (`GameplayStatics.GetGameMode`)))
  (set `self.Gamemode` _asspace_invaders_game_mode)
  (if (`self.Fire`)
    (`/Engine/EditorBlueprintResources/StandardMacros.DoOnce` false :!label _label
      (:`Completed`
        (`|SpawnActorFromClass` "/Game/Blueprints/PlayerProjectile_BP.PlayerProjectile_BP_C" (`KismetMathLibrary.MakeTransform` (`self.K2_GetActorLocation`) (struct) (0.25 1.0 2.5)) "AlwaysSpawn" "OverrideRootScale")
        (`KismetSystemLibrary.Delay` 0.5)
        (goto _label :!via `Reset`)))))

(event `self.ReceiveBeginPlay`
  (set `self.Speed` 600.0))

(event `self.Trigger.OnComponentBeginOverlap`
  (params (OverlappedComponent :type "PrimitiveComponent Object Reference") (OtherActor :type "Actor Object Reference") (OtherComp :type "PrimitiveComponent Object Reference") (OtherBodyIndex :type Integer) (bFromSweep :type Boolean) (SweepResult :type "HitResult Structure (by ref)"))
  (bind _asalien_projectile_bp (cast `/Game/Blueprints/AlienProjectile_BP` OtherActor))
  (`|SpawnActorFromClass` "/Game/Blueprints/PlayerExplosion_BP.PlayerExplosion_BP_C" (`KismetMathLibrary.MakeTransform` (`self.K2_GetActorLocation`) (struct) (1.5 1.5 1.5)) "AdjustIfPossibleButDontSpawnIfColliding" "OverrideRootScale")
  (`self.K2_DestroyActor`)
  (`self.K2_DestroyActor` _asalien_projectile_bp))

(fn `UserConstructionScript`)