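; Alien projectile actor that flies at a fixed speed set on its projectile movement component at BeginPlay.
; When its trigger stops overlapping a top/down trigger flagged as the down one, it spawns an alien explosion at its location, tints the sprite red and destroys itself.
; This ends shots once they leave through the bottom boundary trigger.
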(event `self.ReceiveBeginPlay`
  (bind _projectilemovement1 (`self.ProjectileMovement1`))
  (set `ProjectileMovementComponent.InitialSpeed` 1000.0 _projectilemovement1)
  (set `ProjectileMovementComponent.MaxSpeed` 1000.0 _projectilemovement1))

(event `self.Trigger.OnComponentEndOverlap`
  (params (OtherActor :type "Actor Object Reference") (OtherComp :type "PrimitiveComponent Object Reference") (OtherBodyIndex :type Integer))
  (bind _astop_down_trigger_bp (cast `/Game/Blueprints/TopDownTrigger_BP` OtherActor))
  (if (`/Game/Blueprints/TopDownTrigger_BP.IsDownTrigger?` _astop_down_trigger_bp)
    (bind _returnvalue (`|SpawnActorFromClass` "/Game/Blueprints/AlienExplosion_BP.AlienExplosion_BP_C" (`KismetMathLibrary.MakeTransform` (`self.K2_GetActorLocation`) (struct)) true))
    (`PaperSpriteComponent.SetSpriteColor` _returnvalue (struct :`R` 1.0 :`A` 1.0))
    (`self.K2_DestroyActor`)))

(fn `UserConstructionScript`)