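; Main game actor for a Space Invaders clone that spawns the player, alien waves, shields, edge triggers and HUD, and owns the fixed camera.
; Tick moves the player from GameMode input and runs a DoOnce-gated loop that steps alien rows with staggered delays, reverses and descends at limits, and fires random aliens.
; Destroyed-actor bindings drive lives, respawn, game over, wave speed-up and next-wave spawning.
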(event `SpawnPlayer`
  ;[0 1 0] Player Events
  ;;[1 1 1] Player Events
  (bind _returnvalue (`|SpawnActorFromClass` "/Game/Blueprints/Player_BP.Player_BP_C" (`KismetMathLibrary.MakeTransform` (`KismetMathLibrary.MakeVector` (* (+ (`self.Spacing`) -1100.0) -1.0) 0.0 (* (`self.Spacing`) -3.0)) (struct)) "AdjustIfPossibleButDontSpawnIfColliding" "OverrideRootScale"))
  (bind _output_get (set `self.Player_ref` _returnvalue))
  (add `self.OnDestroyed` _output_get (delegate `PlayerDeathEvent`))
  (set `/Game/Blueprints/Player_BP.Clamp_X_Location` (`KismetMathLibrary.MakeVector2D` (`self.Min_X`) (`self.Max_X`)) _output_get)
  (`KismetSystemLibrary.Delay` 0.2)
  (set `self.PlayerIsDead` false))

(event `VariablesInitialization`
  ;[1 1 1] Variables Initialization Event
  (set `self.GameOver` false)
  (set `self.Score` 0)
  (set `self.Lives` 3)
  (set `self.Spacing` 200.0)
  (set `self.Min_X` (* (`self.Spacing`) -1.0))
  (set `self.Max_X` (* (`self.Spacing`) 11.0))
  (set `self.H_Movement_Direction` 1)
  (set `self.X_Offset_Temp` 0.0)
  (set `self.Z_Offset_Temp` 0.0)
  (set `self.Wave_Horizontal_Speed` 30.0)
  (set `self.Wave_Vertical_Speed` 40.0)
  (set `self.Delay` 0.05)
  (set `self.FireRate` 2.0))

(event `SpawnAlienWaves`
  ;[1 0 0] Aliens Events
  ;;[1 1 1] Spawn Aliens Wave
  (for _index (range 5)
    (for _index_2 (range 11)
      (bind _returnvalue (`KismetMathLibrary.MakeVector` (+ (* _index_2 (`self.Spacing`)) (`self.Min_X`)) 0.0 (* (+ _index 2) (`self.Spacing`))))
      (bind _returnvalue_2 (`|SpawnActorFromClass` "/Game/Blueprints/Alien_BP.Alien_BP_C" (`KismetMathLibrary.MakeTransform` _returnvalue (struct) (1.0 1.0 1.0)) "AlwaysSpawn" "OverrideRootScale"))
      (add `self.OnDestroyed` _returnvalue_2 (delegate `AlienDeathEvent`))
      (set `/Game/Blueprints/Alien_BP.Start_Location` _returnvalue _returnvalue_2)
      (switch `int` _index
        (:`0`
          (set `/Game/Blueprints/Alien_BP.Score` 10 _returnvalue_2)
          (`PaperFlipbookComponent.SetFlipbook` _returnvalue_2 "/Game/Flipbooks/E1_Flipbook.E1_Flipbook")
          (`KismetArrayLibrary.Array_Add` (`self.AliensRow1Array`) _returnvalue_2))
        (:`1`
          (set `/Game/Blueprints/Alien_BP.Score` 15 _returnvalue_2)
          (`PaperFlipbookComponent.SetFlipbook` _returnvalue_2 "/Game/Flipbooks/E2_Flipbook.E2_Flipbook")
          (`KismetArrayLibrary.Array_Add` (`self.AliensRow2Array`) _returnvalue_2))
        (:`2`
          (set `/Game/Blueprints/Alien_BP.Score` 20 _returnvalue_2)
          (`PaperFlipbookComponent.SetFlipbook` _returnvalue_2 "/Game/Flipbooks/E3_Flipbook.E3_Flipbook")
          (`KismetArrayLibrary.Array_Add` (`self.AliensRow3Array`) _returnvalue_2))
        (:`3`
          (set `/Game/Blueprints/Alien_BP.Score` 25 _returnvalue_2)
          (`PaperFlipbookComponent.SetFlipbook` _returnvalue_2 "/Game/Flipbooks/E4_Flipbook.E4_Flipbook")
          (`KismetArrayLibrary.Array_Add` (`self.AliensRow4Array`) _returnvalue_2))
        (:`4`
          (set `/Game/Blueprints/Alien_BP.Score` 30 _returnvalue_2)
          (`PaperFlipbookComponent.SetFlipbook` _returnvalue_2 "/Game/Flipbooks/E5_Flipbook.E5_Flipbook")
          (`KismetArrayLibrary.Array_Add` (`self.AliensRow5Array`) _returnvalue_2))))))

(event `PlayerDeathEvent`
  (params (DestroyedActor :type "Actor Object Reference"))
  ;[0 1 0] Player Events
  ;;[1 1 1] Player Events
  (`self.UpdateLives` 1)
  (set `self.PlayerIsDead` true)
  (if (> (`self.Lives`) 0)
    (`KismetSystemLibrary.Delay` 1.0)
    (`self.SpawnPlayer`)
    (else
      (`|SpawnActorFromClass` "/Game/Blueprints/PlayerExplosion_BP.PlayerExplosion_BP_C" (`KismetMathLibrary.Conv_VectorToTransform` (`self.K2_GetActorLocation` (`self.Player_ref`))) "AdjustIfPossibleButDontSpawnIfColliding" "OverrideRootScale")
      (`self.Game Over Event`))))

(event `ConfigMainGameCamera`
  ;[1 1 1] Config Camera Event
  (`SceneComponent.K2_SetWorldLocationAndRotation` (`self.MainCamera`) (`KismetMathLibrary.MakeVector` (* (`self.Spacing`) 11.0 0.5) 200.0 (* (`self.Spacing`) 5.0 0.5)) (struct :`Yaw` -90.0) false false)
  (`PlayerController.SetViewTargetWithBlend` (`GameplayStatics.GetPlayerController` 0) self 0.0 "VTBlend_Linear" 0.0 false))

(event `SpawnTopDownTrigger`
  ;[0 1 0] Player Events
  ;;[1 1 1] Spawn Top/Down Trigger Events
  (bind _returnvalue (`|SpawnActorFromClass` "/Game/Blueprints/TopDownTrigger_BP.TopDownTrigger_BP_C" (`KismetMathLibrary.MakeTransform` (`KismetMathLibrary.MakeVector` (* (`self.Spacing`) 11.0 0.5) 0.0 (* (`self.Spacing`) -3.0))) "AlwaysSpawn" "OverrideRootScale"))
  (set `/Game/Blueprints/TopDownTrigger_BP.IsDownTrigger?` true _returnvalue)
  (`BoxComponent.SetBoxExtent` _returnvalue (`KismetMathLibrary.MakeVector` (* (`self.Spacing`) 11.0) 10.0 40.0) true)
  (bind _returnvalue_2 (`|SpawnActorFromClass` "/Game/Blueprints/TopDownTrigger_BP.TopDownTrigger_BP_C" (`KismetMathLibrary.MakeTransform` (`KismetMathLibrary.MakeVector` (* (`self.Spacing`) 11.0 0.5) 0.0 (* (`self.Spacing`) 8.0))) "AlwaysSpawn" "OverrideRootScale"))
  (set `/Game/Blueprints/TopDownTrigger_BP.IsDownTrigger?` false _returnvalue_2)
  (`BoxComponent.SetBoxExtent` _returnvalue_2 (`KismetMathLibrary.MakeVector` (* (`self.Spacing`) 11.0) 10.0 40.0) true))

(event `UpdateScore`
  (params (Value :type Integer :default 0))
  ;[1 1 1] Update Score
  (bind _output_get (set `self.Score` (+ (`self.Score`) Value)))
  (`/Game/Blueprints/Widgets_BP/HUD_WG_BP.UpdateScore` (`self.HUD_WG_ref`) _output_get))

(event `AlienDeathEvent`
  (params (DestroyedActor :type "Actor Object Reference"))
  ;[1 0 0] Aliens Events
  ;;[1 1 1] Alien Death Event
  (set `self.Wave_Horizontal_Speed` (`KismetMathLibrary.FClamp` (+ (`self.Wave_Horizontal_Speed`) 2.0) 30.0 80.0))
  (set `self.Delay` (`KismetMathLibrary.FClamp` (- (`self.Delay`) 0.0005) 0.035 0.05))
  (`self.CheckNextWave`))

(event `UpdateLives`
  (params (Value :type Integer :default 0))
  ;[1 1 1] Update Lives
  (bind _output_get (set `self.Lives` (`KismetMathLibrary.Clamp` (- (`self.Lives`) Value) 0 3)))
  (bind _output_get_2 (set `/Game/Blueprints/SpaceInvaders_GameMode.Lives` _output_get (`self.GameMode_Ref`)))
  (`/Game/Blueprints/Widgets_BP/HUD_WG_BP.UpdateLives` (`self.HUD_WG_ref`) _output_get_2))

(event `SpawnProtectors`
  ;[0 1 0] Player Events
  ;;[1 1 1] Spawn Protectors Event
  (for _index (range 4)
    (`|SpawnActorFromClass` "/Game/Blueprints/Protector_BP.Protector_BP_C" (`KismetMathLibrary.MakeTransform` (`KismetMathLibrary.MakeVector` (- (* (* _index 3) (`self.Spacing`)) (/ (`self.Spacing`) 2.0)) 0.0 (* (`self.Spacing`) -2.0))) "AlwaysSpawn" "OverrideRootScale")))

(event `HorizontalMovementEvent`
  (params (AliensRowArray :type "Array of /Game/Blueprints/Alien_BP Object Reference"))
  ;[1 0 0] Aliens Events
  ;;[1 1 1] Row Horizontal Movement Event
  (for _array_element AliensRowArray
    (`/Engine/EditorBlueprintResources/StandardMacros.IsValid` _array_element
      (:`Is Valid`
        (bind (_start_location_x _start_location_y _start_location_z) (`KismetMathLibrary.BreakVector` (`/Game/Blueprints/Alien_BP.Start_Location` _array_element)))
        (`self.K2_SetActorLocation` _array_element (`KismetMathLibrary.MakeVector` (+ _start_location_x (`self.X_Offset_Temp`)) _start_location_y (+ _start_location_z (+ (`self.Spacing`) (`self.Z_Offset_Temp`)))) false false)))))

(event `Game Over Event`
  ;[1 1 1] Game Over Event
  (set `self.GameOver` true)
  (`/Game/Blueprints/Widgets_BP/HUD_WG_BP.GameOver` (`self.HUD_WG_ref`))
  (`KismetSystemLibrary.Delay` 0.0)
  (`GameplayStatics.OpenLevel` "MainGameMap"))

(event `KillPlayerEvent`
  ;[0 1 0] Player Events
  ;;[1 1 1] Kill Player Event
  (`self.UpdateLives` 3)
  (`KismetSystemLibrary.Delay` 0.1)
  (`self.K2_DestroyActor` (`self.Player_ref`)))

(event `RandomFiringEvent`
  (params (Count :type Integer))
  ;[1 0 0] Aliens Events
  ;;[1 1 1] Random Firing Event
  (bind _outactors (`GameplayStatics.GetAllActorsOfClass` "/Game/Blueprints/Alien_BP.Alien_BP_C"))
  (bind _output_get (set `self.AliensArrayTemp` _outactors))
  (`/Engine/EditorBlueprintResources/StandardMacros.CompareInt` (`KismetArrayLibrary.Array_Length` _output_get)
    (:`>`
      (for _ (range 1 (+ Count 1))
        (bind _output_get_2 (set `self.Selected_Alien_Temp` (`KismetMathLibrary.RandomIntegerInRange` 0 (- (`KismetArrayLibrary.Array_Length` (`self.AliensArrayTemp`)) 1))))
        (`/Game/Blueprints/Alien_BP.Fire` (`KismetArrayLibrary.Array_Get` (`self.AliensArrayTemp`) _output_get_2))
        (`KismetArrayLibrary.Array_Remove` (`self.AliensArrayTemp`) (`self.Selected_Alien_Temp`))))))

(event `CheckNextWave`
  ;[1 0 0] Aliens Events
  ;;[1 1 1] Check if All Aliens Are Dead then Spawn Next Wave
  (bind _outactors (`GameplayStatics.GetAllActorsOfClass` "/Game/Blueprints/Alien_BP.Alien_BP_C"))
  (if (not (> (`KismetArrayLibrary.Array_Length` _outactors) 1))
    (`self.UpdateScore` 1000)
    (`self.UpdateLives` 1)
    (set `self.Z_Offset_Temp` 0.0)
    (`self.SpawnAlienWaves`)))

(event `self.ReceiveBeginPlay`
  ;[0 0.4666 1] Begin Play Event
  (bind _asspace_invaders_game_mode (cast `/Game/Blueprints/SpaceInvaders_GameMode` (`GameplayStatics.GetGameMode`)))
  (set `self.GameMode_Ref` _asspace_invaders_game_mode)
  (`self.VariablesInitialization`)
  (`self.ConfigMainGameCamera`)
  (set `/Game/Blueprints/SpaceInvaders_GameMode.Lives` 3 _asspace_invaders_game_mode)
  (`self.SpawnPlayer`)
  (`self.SpawnAlienWaves`)
  (`self.SpawnTopDownTrigger`)
  (`self.SpawnProtectors`)
  (bind _returnvalue (`|CreateWidget` "/Game/Blueprints/Widgets_BP/HUD_WG_BP.HUD_WG_BP_C"))
  (bind _output_get (set `self.HUD_WG_ref` _returnvalue))
  (`UserWidget.AddToViewport` _output_get 0)
  (`self.UpdateLives` 0)
  (`self.UpdateScore` 0))

(event `SpeedUpMovementEvent`
  ;[1 0 0] Aliens Events
  ;;[1 1 1] Speed Up Horizontal Movement
  (set `self.Wave_Horizontal_Speed` (`KismetMathLibrary.FClamp` (+ (`self.Wave_Horizontal_Speed`) 1.0) 30.0 100.0))
  (set `self.Delay` (`KismetMathLibrary.FClamp` (- (`self.Delay`) 0.0005) 0.03 0.05)))

(event `UpdateMovement`
  ;[0 1 0.241] Tick Event
  (bind _outactors (`GameplayStatics.GetAllActorsOfClass` "/Game/Blueprints/Alien_BP.Alien_BP_C" :!label _label))
  (set `/Game/Blueprints/SpaceInvaders_GameMode.AliveEnemies` (`KismetArrayLibrary.Array_Length` _outactors) (`self.GameMode_Ref`))
  (`self.HorizontalMovementEvent` (`self.AliensRow1Array`))
  (`KismetSystemLibrary.Delay` (`self.Delay`))
  (`self.HorizontalMovementEvent` (`self.AliensRow2Array`))
  (`KismetSystemLibrary.Delay` (`self.Delay`))
  (`self.HorizontalMovementEvent` (`self.AliensRow3Array`))
  (`KismetSystemLibrary.Delay` (`self.Delay`))
  (`self.HorizontalMovementEvent` (`self.AliensRow4Array`))
  (`KismetSystemLibrary.Delay` (`self.Delay`))
  (`self.HorizontalMovementEvent` (`self.AliensRow5Array`))
  (`KismetSystemLibrary.Delay` (`self.Delay`))
  (if (and (> (`self.X_Offset_Temp`) (* (`self.Spacing`) 1.5)) (== (`self.H_Movement_Direction`) 1))
    (set `self.H_Movement_Direction` -1) ; Change Direction : Move Left
    (set `self.Z_Offset_Temp` (- (`self.Z_Offset_Temp`) (`self.Wave_Vertical_Speed`)) :!label _label_2)
    (`KismetSystemLibrary.Delay` (* (`self.Delay`) 5.0))
    (`self.UpdateMovement`)
    (elif (and (< (`self.X_Offset_Temp`) 0.0) (== (`self.H_Movement_Direction`) -1))
      (set `self.H_Movement_Direction` 1) ; Change Direction : Move Right
      (goto _label_2)
      (else
        (`self.ResetMovementDoOnce`)))))

(event `self.ReceiveTick`
  (params (DeltaSeconds :type "Float (single-precision)"))
  (bind _gamemode_ref (`self.GameMode_Ref`))
  (bind _returnvalue (`self.K2_GetActorLocation` (`self.Player_ref`)))
  (bind (_clamp_x_location_x _clamp_x_location_y) (`KismetMathLibrary.BreakVector2D` (`/Game/Blueprints/Player_BP.Clamp_X_Location` (`self.Player_ref`))))
  (bind _returnvalue_x (`KismetMathLibrary.BreakVector` (+ (* (1.0 0.0 0.0) (* (`/Game/Blueprints/SpaceInvaders_GameMode.MovementDirection` (`self.GameMode_Ref`)) (`/Game/Blueprints/Player_BP.Speed` (`self.Player_ref`)) (`GameplayStatics.GetWorldDeltaSeconds`) -1.0)) _returnvalue)))
  ;[0 1 0.241] Tick Event
  (`/Engine/EditorBlueprintResources/StandardMacros.IsValid` _gamemode_ref
    (:`Is Valid`
      (if (and (`/Game/Blueprints/SpaceInvaders_GameMode.GameStarted` _gamemode_ref) (not (`self.PlayerIsDead`)))
        (set `/Game/Blueprints/Player_BP.Fire` (`/Game/Blueprints/SpaceInvaders_GameMode.Fire` (`self.GameMode_Ref`)) (`self.Player_ref`))
        (`self.K2_SetActorLocation` (`self.Player_ref`) (`KismetMathLibrary.MakeVector` (`KismetMathLibrary.FClamp` _returnvalue_x _clamp_x_location_x _clamp_x_location_y) (.y _returnvalue) (.z _returnvalue)) true false)
        (`/Engine/EditorBlueprintResources/StandardMacros.DoOnce` false :!label _label_3
          (:`Completed`
            (`|ExecutionSequence`
              (:`then_0`
                (set `self.X_Offset_Temp` (+ (`self.X_Offset_Temp`) (* (`self.H_Movement_Direction`) (`self.Wave_Horizontal_Speed`))))
                (goto _label))
              (:`then_1`
                (`KismetSystemLibrary.Delay` (`self.FireRate`))
                (`self.RandomFiringEvent` (`KismetMathLibrary.RandomIntegerInRange` 1 4))))))))))

(event `ResetMovementDoOnce`
  ;[0 1 0.241] Tick Event
  (goto _label_3 :!via `Reset`))

(fn `UserConstructionScript`)