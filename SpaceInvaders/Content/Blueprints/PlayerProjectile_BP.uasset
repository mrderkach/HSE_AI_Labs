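; PlayerProjectile_BP is the player's shot in what appears to be an alien shooter, moving at a fixed speed set on its projectile movement component.
; Its Trigger overlap destroys aliens or alien projectiles along with itself, spawning an explosion at the hit, scaled down for projectiles.
; Leaving a TopDownTrigger not marked as the down trigger destroys it with a red-tinted explosion.
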(event `self.ReceiveBeginPlay`
  (bind _projectilemovement1 (`self.ProjectileMovement1`))
  (set `ProjectileMovementComponent.InitialSpeed` 2000.0 _projectilemovement1)
  (set `ProjectileMovementComponent.MaxSpeed` 2000.0 _projectilemovement1))

(event `self.Trigger.OnComponentBeginOverlap`
  (params (OtherActor :type "Actor Object Reference") (OtherComp :type "PrimitiveComponent Object Reference") (OtherBodyIndex :type Integer) (bFromSweep :type Boolean) (SweepResult :type "EngineTypes.HitResult Structure (by ref)"))
  (bind _asalien_bp (cast `/Game/Blueprints/Alien_BP` OtherActor)
    (:`then`
      (`self.K2_DestroyActor`)
      (`|SpawnActorFromClass` "/Game/Blueprints/AlienExplosion_BP.AlienExplosion_BP_C" (`KismetMathLibrary.MakeTransform` (`self.K2_GetActorLocation` _asalien_bp)) true)
      (`self.K2_DestroyActor` _asalien_bp))
    (:`CastFailed`
      (bind _asalien_projectile_bp (cast `/Game/Blueprints/AlienProjectile_BP` OtherActor))
      (`self.K2_DestroyActor`)
      (`|SpawnActorFromClass` "/Game/Blueprints/AlienExplosion_BP.AlienExplosion_BP_C" (`KismetMathLibrary.MakeTransform` (`self.K2_GetActorLocation` _asalien_projectile_bp) (struct) (0.25 0.25 0.25)) true)
      (`self.K2_DestroyActor` _asalien_projectile_bp))))

(event `self.Trigger.OnComponentEndOverlap`
  (params (OtherActor :type "Actor Object Reference") (OtherComp :type "PrimitiveComponent Object Reference") (OtherBodyIndex :type Integer))
  (bind _astop_down_trigger_bp (cast `/Game/Blueprints/TopDownTrigger_BP` OtherActor))
  (if (not (`/Game/Blueprints/TopDownTrigger_BP.IsDownTrigger?` _astop_down_trigger_bp))
    (bind _returnvalue (`|SpawnActorFromClass` "/Game/Blueprints/AlienExplosion_BP.AlienExplosion_BP_C" (`KismetMathLibrary.MakeTransform` (`self.K2_GetActorLocation`) (struct)) true))
    (`PaperSpriteComponent.SetSpriteColor` _returnvalue (struct :`R` 1.0 :`A` 1.0))
    (`self.K2_DestroyActor`)))

(fn `UserConstructionScript`)