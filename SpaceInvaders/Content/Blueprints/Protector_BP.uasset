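; Protector builds a block structure out of individual ProtectorPart_BP actors when play begins.
; Nested loops spawn the parts on an evenly spaced grid in the X-Z plane, offset from the actor's location.
; A condition skips the middle columns of the two lowest rows, leaving an arch-like notch between two legs.
; Parts always spawn regardless of collision, and the construction script is empty.
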(event `self.ReceiveBeginPlay`
  (set `self.Spacing` 25.0)
  (for _index (range 7)
    (for _index_2 (range 9)
      (if (not (and (> _index_2 1) (< _index_2 7) (< _index 2)))
        (`|SpawnActorFromClass` "/Game/Blueprints/ProtectorPart_BP.ProtectorPart_BP_C" (`KismetMathLibrary.MakeTransform` (+ (`KismetMathLibrary.MakeVector` (* _index_2 (`self.Spacing`)) 0.0 (* _index (`self.Spacing`))) (`self.K2_GetActorLocation`))) "AlwaysSpawn" "OverrideRootScale")))))

(fn `UserConstructionScript`)